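; BP_Ghost is an AI-controlled ghost that can be stunned and captured.
; Its Stun and Capture events each set a boolean key (Stuned or Capture) to true on its AI controller's Blackboard; nothing here clears them.
; Tick caches the frame's delta seconds in DeltaTime, and the construction script is empty.
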(event Custom|Stun
  (AI|Components|Blackboard|SetValueasBool (AI|GetBlackboard (AI|GetAIController self)) (Utilities|Name|MakeLiteralName "Stuned") true))

(event Custom|Capture
  (AI|Components|Blackboard|SetValueasBool (AI|GetBlackboard (AI|GetAIController self)) (Utilities|Name|MakeLiteralName "Capture") true))

(event EventTick
  (params (DeltaSeconds :type Float%20%28single-precision%29))
  (Variables|Default|SetDeltaTime DeltaSeconds))

(fn ConstructionScript)